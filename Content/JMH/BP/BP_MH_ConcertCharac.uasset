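; BP_MH_ConcertCharac is a concert character actor that moves its root vertically once play begins.
; A Timeline started on BeginPlay drives a Z lerp between offsets below and above the root's position, set by SubVarA and AddVarB.
; Each update re-reads the current world location and writes it as relative location, so the offsets follow the moving root rather than a stored start point.
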(event `self.ReceiveBeginPlay`
  (bind (_returnvalue_x _returnvalue_y _returnvalue_z) (`KismetMathLibrary.BreakVector` (`SceneComponent.K2_GetComponentLocation` (`self.DefaultSceneRoot`))))
  (bind (_direction _newtrack_0) (`Timeline|Timeline` :`NewTime` (`self.New Time`))
    (:`Update`
      (`SceneComponent.K2_SetRelativeLocation` (`self.DefaultSceneRoot`) (`KismetMathLibrary.MakeVector` _returnvalue_x _returnvalue_y (`KismetMathLibrary.Lerp` (- _returnvalue_z (`self.SubVarA`)) (+ _returnvalue_z (`self.AddVarB`)) _newtrack_0)) false false))))

(fn `UserConstructionScript`)