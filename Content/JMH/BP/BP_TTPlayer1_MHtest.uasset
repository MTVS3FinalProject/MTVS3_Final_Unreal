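; BP_TTPlayer1_MHtest is a player Blueprint, apparently a test variant, that plays rocket-style feedback for a chair going up.
; PlayChairGoingUpCameraShake plays a world camera shake at the player's location, then calls a server event that hands off to a multicast, which plays two rocket sound cues there.
; Unconnected nodes that look up the hall sound manager and throw the lucky draw chair never run.
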(event `self.ReceiveBeginPlay`)

(event `Key|Q`
  (params (Key :type "Key Structure")))

(event `self.PlayChairGoingUpCameraShake`
  (`GameplayStatics.PlayWorldCameraShake` "/Game/KHJ/Camera/BP_LegacyCameraShake.BP_LegacyCameraShake_C" (`self.K2_GetActorLocation`) 0.0 3000.0)
  (`self.ServerPlayGoingUpSound`))

(event `ServerPlayGoingUpSound`
  (`self.MulticastPlayGoingUpSound`))

(event `MulticastPlayGoingUpSound`
  (bind _returnvalue (`self.K2_GetActorLocation`))
  (`GameplayStatics.PlaySoundAtLocation` "/Game/KHJ/Assets/Sounds/A_RocketCameraShake_Cue.A_RocketCameraShake_Cue" _returnvalue (struct) 1.0 1.0 0.0 null null null null)
  (`GameplayStatics.PlaySoundAtLocation` "/Game/KHJ/Assets/Sounds/A_Rocket_Cue.A_Rocket_Cue" _returnvalue (struct) 1.0 1.0 0.0 null null null null))

(fn `UserConstructionScript`)