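; Trigger actor that teleports an overlapping TTPlayer toward the concert hall.
; On begin overlap it calls the player's ServerTeleportPlayer, sets the game instance place state to ConcertHall and starts concert BGM.
; End overlap would teleport player and lucky-draw chair to a hard-coded spot, but casts one actor to both classes, so likely never fires.
; Leftover level-streaming and teleport nodes are unconnected.
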(event `self.ReceiveActorBeginOverlap`
  (params (OtherActor :type "Actor Object Reference"))
  (bind _asttplayer (cast `TTPlayer` OtherActor))
  (`TTPlayer.ServerTeleportPlayer` _asttplayer true)
  (bind _asttgame_instance (cast `TTGameInstance` (`GameplayStatics.GetGameInstance`)))
  (`TTGameInstance.SetPlaceState` _asttgame_instance "ConcertHall")
  (`TTPlayer.PlayConcertBGM` _asttplayer))

(event `self.ReceiveActorEndOverlap`
  (params (OtherActor :type "Actor Object Reference"))
  (bind _asbp_lucky_draw_chair (cast `/Game/KHJ/Blueprints/BP_LuckyDrawChair` OtherActor))
  (bind _asbp_ttplayer (cast `/Game/KHJ/Blueprints/BP_TTPlayer` OtherActor))
  (`self.ServerTeleport` _asbp_ttplayer _asbp_lucky_draw_chair))

(event `ServerTeleport`
  (params (TTPlayer :type "/Game/KHJ/Blueprints/BP_TTPlayer Object Reference") (LuckyDrawChair :type "/Game/KHJ/Blueprints/BP_LuckyDrawChair Object Reference"))
  (`self.K2_TeleportTo` :`self` TTPlayer :`DestLocation` (530.0 10650.0 940.0))
  (`self.K2_TeleportTo` :`self` LuckyDrawChair :`DestLocation` (530.0 10650.0 940.0)))

(fn `UserConstructionScript`)