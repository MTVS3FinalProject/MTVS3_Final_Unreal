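; Teleport trigger actor that sends an overlapping player toward the Plaza state.
; On begin overlap it casts to TTPlayer and calls ServerTeleportPlayer, leaving the destination to that function.
; It then sets the game instance's place state to Plaza and calls the player's PlayConcertBGM, with no local-control check.
; Disconnected nodes hold unused level streaming and hard-coded teleport experiments that never run.
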(event `self.ReceiveActorBeginOverlap`
  (params (OtherActor :type "Actor Object Reference"))
  (bind _asttplayer (cast `TTPlayer` OtherActor))
  (`TTPlayer.ServerTeleportPlayer` _asttplayer true)
  (bind _asttgame_instance (cast `TTGameInstance` (`GameplayStatics.GetGameInstance`)))
  (`TTGameInstance.SetPlaceState` _asttgame_instance "Plaza")
  (`TTPlayer.PlayConcertBGM` _asttplayer))

(event `self.ReceiveActorEndOverlap`
  (params (OtherActor :type "Actor Object Reference")))

(fn `UserConstructionScript`)