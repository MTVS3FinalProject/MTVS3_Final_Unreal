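; BP_HJChair1 is a folding chair actor that shows players whether it is available and in use.
; RotateChair changes the chair mesh's rotation by sitting state, and ChangeLightColor swaps a seat material between green (available) and red.
; Overlap by a locally controlled TTPlayer swaps both meshes' overlay material to an outline, restored on exit.
; A Server-to-Multicast event pair duplicates the color change, but its authority-switch caller is disconnected.
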(event `self.ReceiveBeginPlay`)

(event `self.RotateChair`
  (params (bIsSitting :type Boolean))
  (bind _object_1f_foldingchair (`self.Object_1F_FoldingChair`))
  (if bIsSitting
    (`SceneComponent.K2_SetRelativeRotation` _object_1f_foldingchair (struct :`Yaw` -90.0) false false)
    (else
      (`SceneComponent.K2_SetRelativeRotation` _object_1f_foldingchair (struct :`Pitch` -90.0 :`Yaw` 450.0 :`Roll` -540.0) false false))))

(event `self.ReceiveActorBeginOverlap`
  (params (OtherActor :type "Actor Object Reference"))
  (bind _asttplayer (cast `TTPlayer` OtherActor))
  (if (`Pawn.IsLocallyControlled` _asttplayer)
    (`MeshComponent.SetOverlayMaterial` (`self.Object_1F_FoldingChair_Seat`) "/Game/KHJ/Materials/M_Outline.M_Outline")
    (`MeshComponent.SetOverlayMaterial` (`self.Object_1F_FoldingChair`) "/Game/KHJ/Materials/M_Outline.M_Outline")))

(event `self.ReceiveActorEndOverlap`
  (params (OtherActor :type "Actor Object Reference"))
  (bind _asttplayer (cast `TTPlayer` OtherActor))
  (if (`Pawn.IsLocallyControlled` _asttplayer)
    (`MeshComponent.SetOverlayMaterial` (`self.Object_1F_FoldingChair_Seat`) "/Engine/Functions/Engine_MaterialFunctions02/ExampleContent/3dParticleOpacity_Mat.3dParticleOpacity_Mat")
    (`MeshComponent.SetOverlayMaterial` (`self.Object_1F_FoldingChair`) "/Engine/Functions/Engine_MaterialFunctions02/ExampleContent/3dParticleOpacity_Mat.3dParticleOpacity_Mat")))

(event `self.ChangeLightColor`
  (params (bAvailable :type Boolean))
  (if bAvailable
    ;[1 1 1] 초록색
    (`PrimitiveComponent.SetMaterial` (`self.Object_1F_FoldingChair_Seat`) 2 "/Game/KJM/Materials/M_Chair_Light.M_Chair_Light")
    (else
      ;[1 1 1] 빨간색
      (`PrimitiveComponent.SetMaterial` (`self.Object_1F_FoldingChair_Seat`) 2 "/Game/KJM/Materials/MI_Chair_Light_Red.MI_Chair_Light_Red"))))

(event `ServerChangeLightColor`
  (params (Available :type Boolean))
  (`self.MulticastChangeLightColor` Available))

(event `MulticastChangeLightColor`
  (params (Available :type Boolean))
  (if Available
    ;[1 1 1] 초록색
    (`PrimitiveComponent.SetMaterial` (`self.Object_1F_FoldingChair_Seat`) 2 "/Game/KJM/Materials/M_Chair_Light.M_Chair_Light")
    (else
      ;[1 1 1] 빨간색
      (`PrimitiveComponent.SetMaterial` (`self.Object_1F_FoldingChair_Seat`) 2 "/Game/KJM/Materials/MI_Chair_Light_Red.MI_Chair_Light_Red"))))

(fn `UserConstructionScript`)