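; BP_LuckyDrawChair is a chair actor, named for a lucky draw, that moves vertically with a Niagara effect when ThrowChair is called.
; After a short delay, the event shows the effect and plays a timeline that lerps Z from the current location toward EndLocZ, so steps compound.
; A Delay chained to the timeline's Update later hides the effect and stops the timeline.
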(event `self.ReceiveBeginPlay`)

(event `self.ThrowChair`
  (bind (_returnvalue_x _returnvalue_y) (`KismetMathLibrary.BreakVector` (`self.K2_GetActorLocation`)))
  (bind _niagaracomp (`self.NiagaraComp`))
  (`KismetSystemLibrary.Delay` 1.2)
  (`SceneComponent.SetVisibility` _niagaracomp true false)
  (bind (_direction _goingup) (`Timeline|Timeline` :!label _label)
    (:`Update`
      (`self.K2_SetActorLocation` (`KismetMathLibrary.VLerp` (`self.K2_GetActorLocation`) (`KismetMathLibrary.MakeVector` _returnvalue_x _returnvalue_y (`self.EndLocZ`)) _goingup))
      (`KismetSystemLibrary.Delay` 5.0)
      (`SceneComponent.SetVisibility` _niagaracomp false false)
      (goto _label :!via `Stop`))))

(fn `UserConstructionScript`)