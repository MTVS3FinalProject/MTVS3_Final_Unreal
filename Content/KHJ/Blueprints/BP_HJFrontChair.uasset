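; BP_HJFrontChair is a folding chair actor that rotates for sitting and highlights on overlap.
; The RotateChair event takes an IsSitting flag and snaps the Object1FFoldingChair component between two fixed relative rotations, leaving the separate seat component untouched.
; Actor overlap sets an outline overlay material on both chair and seat, and end overlap swaps it for a particle opacity material.
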(event `self.ReceiveBeginPlay`)

(event `self.RotateChair`
  (params (bIsSitting :type Boolean))
  (bind _object_1f_foldingchair (`self.Object_1F_FoldingChair`))
  (if bIsSitting
    (`SceneComponent.K2_SetRelativeRotation` _object_1f_foldingchair (struct :`Yaw` -90.0) false false)
    (else
      (`SceneComponent.K2_SetRelativeRotation` _object_1f_foldingchair (struct :`Pitch` -90.0 :`Yaw` 450.0 :`Roll` -540.0) false false))))

(event `self.ReceiveActorBeginOverlap`
  (params (OtherActor :type "Actor Object Reference"))
  (`MeshComponent.SetOverlayMaterial` (`self.Object_1F_FoldingChair_Seat`) "/Game/KHJ/Materials/M_Outline.M_Outline")
  (`MeshComponent.SetOverlayMaterial` (`self.Object_1F_FoldingChair`) "/Game/KHJ/Materials/M_Outline.M_Outline"))

(event `self.ReceiveActorEndOverlap`
  (params (OtherActor :type "Actor Object Reference"))
  (`MeshComponent.SetOverlayMaterial` (`self.Object_1F_FoldingChair_Seat`) "/Engine/Functions/Engine_MaterialFunctions02/ExampleContent/3dParticleOpacity_Mat.3dParticleOpacity_Mat")
  (`MeshComponent.SetOverlayMaterial` (`self.Object_1F_FoldingChair`) "/Engine/Functions/Engine_MaterialFunctions02/ExampleContent/3dParticleOpacity_Mat.3dParticleOpacity_Mat"))

(fn `UserConstructionScript`)