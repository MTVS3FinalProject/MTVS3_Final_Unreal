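; Lucky draw table actor that provides visual feedback through table material changes and a spark effect.
; SetColorRed, SetColorBlue and SetColorBlack forward to Multicast-named events, which swap the table mesh's first material to red, blue or screen.
; PlaySpark activates the sparks component directly, without a multicast wrapper.
; It has no active logic of its own, only these callable events.
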(event `self.SetColorBlue`
  (`self.MulticastSetColorBlue`))

(event `self.SetColorRed`
  (`self.MulticastSetColorRed`))

(event `MulticastSetColorRed`
  (`PrimitiveComponent.SetMaterial` (`self.TableMeshComp`) 0 "/Game/KHJ/Materials/M_Red.M_Red"))

(event `MulticastSetColorBlue`
  (`PrimitiveComponent.SetMaterial` (`self.TableMeshComp`) 0 "/Game/KHJ/Materials/M_Blue.M_Blue"))

(event `self.SetColorBlack`
  (`self.MulticastSetColorBlack`))

(event `self.PlaySpark`
  (`ActorComponent.Activate` (`self.SparksV2_2`) false))

(event `MulticastSetColorBlack`
  (`PrimitiveComponent.SetMaterial` (`self.TableMeshComp`) 0 "/Game/KJM/Materials/M_Screen.M_Screen"))

(fn `UserConstructionScript`)