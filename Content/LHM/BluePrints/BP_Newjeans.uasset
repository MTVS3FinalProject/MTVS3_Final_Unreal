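; BP_Newjeans is an actor that moves vertically from BeginPlay, apparently intended as a bobbing motion.
; Two timelines drive it, one lerping the actor upward and the other downward by the same small offset.
; Each calls Play on the other from its Update pin rather than Finished, so they run concurrently.
; Both lerps start from the root's current world location, so offsets apply incrementally rather than from a fixed origin.
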(event `self.ReceiveBeginPlay`
  (bind _defaultsceneroot (`self.DefaultSceneRoot`))
  (bind _defaultsceneroot_2 (`self.DefaultSceneRoot`))
  (bind (_returnvalue_x _returnvalue_y _returnvalue_z) (`KismetMathLibrary.BreakVector` (`SceneComponent.K2_GetComponentLocation` _defaultsceneroot_2)))
  (bind (_returnvalue_x_2 _returnvalue_y_2 _returnvalue_z_2) (`KismetMathLibrary.BreakVector` (`SceneComponent.K2_GetComponentLocation` _defaultsceneroot)))
  (bind (_direction _newtrack_1) (`Timeline|Timeline` :!label _label)
    (:`Update`
      (`self.K2_SetActorLocation` (`KismetMathLibrary.VLerp` (`SceneComponent.K2_GetComponentLocation` _defaultsceneroot_2) (`KismetMathLibrary.MakeVector` _returnvalue_x _returnvalue_y (+ _returnvalue_z 5.0)) _newtrack_1))
      (bind (_direction_2 _newtrack_1_2) (`Timeline|Timeline_0`)
        (:`Update`
          (`self.K2_SetActorLocation` (`KismetMathLibrary.VLerp` (`SceneComponent.K2_GetComponentLocation` _defaultsceneroot) (`KismetMathLibrary.MakeVector` _returnvalue_x_2 _returnvalue_y_2 (+ _returnvalue_z_2 -5.0)) _newtrack_1_2))
          (goto _label))))))

(fn `UserConstructionScript`)